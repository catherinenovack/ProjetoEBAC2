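; Master pickup actor that the first-person character can collect, with an empty behavior event as a hook for item-specific effects.
; The construction script reads a data table row into Item and sets the mesh, which spins through a looping Delay from BeginPlay.
; Sphere overlap registers the actor as the character's LastInteractObj and toggles CanInteract.
; Interact, when allowed, calls the hook, destroys the actor and prints an inventory message.
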(event OnComponentBeginOverlap(Sphere)
  (params (OverlappedComponent :type Primitive%20Component%20Object%20Reference) (OtherActor :type Actor%20Object%20Reference) (OtherComp :type Primitive%20Component%20Object%20Reference) (OtherBodyIndex :type Integer) (bFromSweep :type Boolean) (SweepResult :type Hit%20Result%20Structure%20%28by%20ref%29))
  ;[0.15 0.15 0.15 0.5] Entrando na colisão
  (bind _asbp_first_person_character (Utilities|Casting|CastToBP_FirstPersonCharacter OtherActor))
  (Variables|/Game/FirstPerson/Blueprints/BP_FirstPersonCharacter.BP_FirstPersonCharacter_C|SetLastInteractObj _asbp_first_person_character self)
  (Variables|Default|SetCanInteract? true))

(event OnComponentEndOverlap(Sphere)
  (params (OverlappedComponent :type Primitive%20Component%20Object%20Reference) (OtherActor :type Actor%20Object%20Reference) (OtherComp :type Primitive%20Component%20Object%20Reference) (OtherBodyIndex :type Integer))
  ;[0.15 0.15 0.15 0.5] Sem colisão
  (Utilities|Casting|CastToBP_FirstPersonCharacter OtherActor)
  (Variables|Default|SetCanInteract? false))

(event Custom|Variações%20de%20comportamento
  ;[0.15 0.15 0.15 0.5] Interação com o objeto
)

(event EventBeginPlay
  ;[0.15 0.15 0.15 0.5] Rotacionar objeto
  (Transformation|AddLocalRotation (Variables|Default|GetStaticMesh) "0.000000,1.000000,0.000000" false false :!label _label)
  (Utilities|FlowControl|Delay 0.001)
  (goto _label))

(event EventInteract
  ;[0.15 0.15 0.15 0.5] Interação com o objeto
  (if (Variables|Default|GetCanInteract?)
    (CallFunction|VariaçõesDeComportamento)
    (Actor|DestroyActor)
    (Development|PrintString "Adicionado ao inventário")))

(fn ConstructionScript
  (bind _data_table_row_handle (Variables|Default|GetData%20Table%20Row%20Handle))
  (bind (_datatable _rowname) (Utilities|Struct|BreakDataTableRowHandle _data_table_row_handle))
  (bind _returnvalue (Utilities|GetDataTableRow _datatable _rowname)
    (:then
      (bind _output_get (Variables|Default|SetItem _returnvalue))
      (Components|StaticMesh|SetStaticMesh (Variables|Default|GetStaticMesh) (.Mesh (Utilities|Struct|BreakItem_Struct _output_get))))))